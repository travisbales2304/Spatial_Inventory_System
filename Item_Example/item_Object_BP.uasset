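; Item object that holds an item's class, icon and 2D dimensions, with support for a rotated state, as used by grid-style inventories.
; Rotate toggles the Rotated flag, which IsRotated reports.
; GetObjectDimensions swaps X and Y while rotated, and GetIcon returns a separate pre-rotated icon instead of transforming the original.
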(fn `GetIcon`
  (returns (Icon :type "MaterialInterface Object Reference"))
  (if (`self.Rotated`)
    (return (`self.Icon_Rotated`))
    (else
      (return (`self.Icon`)))))

(fn `GetItemClass`
  (returns (ItemClass :type "/Game/Inventory_System/Item_Example/Item_BP Class Reference"))
  (return (`self.ItemClass`)))

(fn `GetObjectDimensions`
  (returns (ObjectDimensions :type "IntPoint Structure"))
  (bind (_objectdimensions_x _objectdimensions_y) (break `IntPoint` (`self.ObjectDimensions`)))
  (if (`self.Rotated`)
    (return (make `IntPoint` _objectdimensions_y _objectdimensions_x))
    (else
      (return (`self.ObjectDimensions`)))))

(fn `IsRotated`
  (returns (Isrotated :type Boolean))
  (return (`self.Rotated`)))

(fn `Rotate`
  (set `self.Rotated` (not (`self.Rotated`))))