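; Item_BP is a world item actor that a player can add to their inventory component.
; On BeginPlay it fills an unset ItemObject from GetDefaultItemObject, which is an empty stub here.
; ServerAddItem passes ItemObject to the player's TryAddItem and destroys the actor on success.
; PrimaryIntereact instead adds a newly fetched default item and returns the result without destroying the actor.
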(event `self.ReceiveBeginPlay`
  (`/Engine/EditorBlueprintResources/StandardMacros.IsValid` (`self.ItemObject`)
    (:`Is Not Valid`
      (bind _itemobject (`self.GetDefaultItemObject`))
      (set `self.ItemObject` _itemobject))))

(event `ServerAddItem`
  (params (PlayerRef :type "/Game/FirstPerson/Blueprints/BP_FirstPersonCharacter Object Reference"))
  (bind _itemadded (`/Game/Inventory_System/Inventory_AC.TryAddItem` (`/Game/FirstPerson/Blueprints/BP_FirstPersonCharacter.Inventory_AC` PlayerRef) (`self.ItemObject`)))
  (if _itemadded
    (`self.K2_DestroyActor`)))

(fn `GetDefaultItemObject`
  (returns (ItemObject :type "/Game/Inventory_System/Item_Example/item_Object_BP Object Reference"))
  (return null))

(fn `Primary_intereact`
  (params (Interactor :type "/Game/FirstPerson/Blueprints/BP_FirstPersonCharacter Object Reference"))
  (returns (Success :type Boolean))
  (bind _itemobject (`self.GetDefaultItemObject`))
  (bind _itemadded (`/Game/Inventory_System/Inventory_AC.TryAddItem` (`/Game/FirstPerson/Blueprints/BP_FirstPersonCharacter.Inventory_AC` Interactor) _itemobject))
  (if _itemadded
    (return true)
    (else
      (return false))))

(fn `UserConstructionScript`)